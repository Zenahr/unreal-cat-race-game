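; Race track manager that sets up a lap-based checkpoint race and tracks its progress.
; On BeginPlay it copies lap count, map, save name and medal times to the player controller, then numbers the checkpoints and binds their cleared events.
; Each clear plays a sound and activates the next checkpoint, updating respawn point and laps.
; After the final lap it flags the race complete and calls the controller's Restart.
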(event `self.ReceiveBeginPlay`
  ;[1 1 1] Event BeginPlay
  ;;[1 1 1] This just sets every other event we do to the player controller. Nothing more, nothing less.
  (bind _asmy_player_controller (cast `/Game/Blueprints/MyPlayerController` (`GameplayStatics.GetPlayerController` 0)))
  (set `self.PlayerControllerReference` _asmy_player_controller)
  (`self.ApplySetings`)
  (`self.StartSequence`))

(event `ApplySetings`
  (bind _playercontrollerreference (`self.PlayerControllerReference`))
  ;[1 1 1] Apply Settings
  (set `/Game/Blueprints/MyPlayerController.MaxLaps` (`self.MaxLaps`) _playercontrollerreference)
  (set `/Game/Blueprints/MyPlayerController.LL_SaveGame` (`self.SaveGameName`) _playercontrollerreference)
  (set `/Game/Blueprints/MyPlayerController.NameOfMap` (`self.NameOfMap`) _playercontrollerreference)
  (`self.UpdateTimes`)
  (`/Game/Blueprints/MyPlayerController.StartGame Setup` _playercontrollerreference))

(event `StartSequence`
  (bind _checkpoints (`self.Checkpoints`))
  ;[1 1 1] Setup Checkpoints logic
  (for (_array_element _array_index) _checkpoints
    (set `/Game/Blueprints/Checkpoint.CheckpointNumber` (+ _array_index 1) _array_element)
    (set `self.TotalCheckpoints` (`KismetArrayLibrary.Array_Length` _checkpoints))
    (`self.ActivateCheckpoint` (`|GetArrayItem` _checkpoints))
    ;[1 1 1] Might be able to chain this to the first for-loop and get rid of the redundancy a bit. Try connecting it to the beginplay chain
    (for _array_element_2 _checkpoints
      (add `/Game/Blueprints/Checkpoint.CheckpointCleared` _array_element_2 (delegate `CheckpointCleared`)))))

(event `CheckpointCleared`
  (params (NextCheckpoint :type Integer))
  (bind _playercontrollerreference (`self.PlayerControllerReference`))
  ;[1 1 1] Might be able to chain this to the first for-loop and get rid of the redundancy a bit. Try connecting it to the beginplay chain
  (`self.LapCheck` NextCheckpoint)
  (`AudioComponent.Play` (`AmbientSound.AudioComponent` (`self.CheckpointSoundFX`)) 0.0)
  ;[1 1 1] Refresh all checkpoints when lap is over
  (if (`/Game/Blueprints/MyPlayerController.RaceComplete` _playercontrollerreference)
    (`/Game/Blueprints/MyPlayerController.Restart` _playercontrollerreference)))

(fn `ActivateCheckpoint`
  (params (NextCheckpoint :type "/Game/Blueprints/Checkpoint Object Reference"))
  (bind _trigger (`/Game/Blueprints/Checkpoint.Trigger` NextCheckpoint))
  ;[1 1 1] Initialize Checkpoint (Make visible)
  (`SceneComponent.SetHiddenInGame` _trigger false false)
  (`SceneComponent.SetHiddenInGame` (`/Game/Blueprints/Checkpoint.ParticleSystem` NextCheckpoint) false false)
  (set `PrimitiveComponent.bGenerateOverlapEvents` true _trigger))

(fn `LapCheck`
  (params (Checkpoint :type Integer))
  (locals (LocalCheckpoint :type Integer))
  (bind _output_get (set `local.LocalCheckpoint` Checkpoint))
  (if (== _output_get (`self.TotalCheckpoints`))
    (bind _isracecomplete_ (`self.RaceCompleteCheck`))
    (if _isracecomplete_
      ;[1 1 1] Update Lap on last lap
      (`/Game/Blueprints/MyPlayerController.UpdateLap` (`self.PlayerControllerReference`))
      (else
        ;[1 1 1] Reactivate first checkpoint
        (`self.ActivateCheckpoint` (`|GetArrayItem` (`self.Checkpoints`)))
        ;[1 1 1] Increment Lap
        (`/Game/Blueprints/MyPlayerController.UpdateLap` (`self.PlayerControllerReference`))
        ;[1 1 1] Set respawn location to previous checkpoint
        (set `/Game/Blueprints/MyPlayerController.RespawnLocation` (`self.GetTransform` (`|GetArrayItem` (`self.Checkpoints`) (- (`local.LocalCheckpoint`) 1))) (`self.PlayerControllerReference`) :!label _label)))
    (else
      (`self.ActivateCheckpoint` (`|GetArrayItem` (`self.Checkpoints`) (`local.LocalCheckpoint`)))
      (goto _label))))

(fn `RaceCompleteCheck`
  (returns (`IsRaceComplete?` :type Boolean))
  (locals (LocalComplete :type Boolean))
  (bind _playercontrollerreference (`self.PlayerControllerReference`))
  (bind _playercontrollerreference_2 (`self.PlayerControllerReference`))
  ;[1 1 1] Race Completion Check
  (if (>= (`/Game/Blueprints/MyPlayerController.ActualLap` _playercontrollerreference_2) (`/Game/Blueprints/MyPlayerController.MaxLaps` _playercontrollerreference_2))
    (bind _output_get (set `/Game/Blueprints/MyPlayerController.RaceComplete` true _playercontrollerreference))
    (set `local.LocalComplete` _output_get)
    (`KismetSystemLibrary.PrintString` "Finished Track!")
    (else
      (bind _output_get_2 (set `/Game/Blueprints/MyPlayerController.RaceComplete` false _playercontrollerreference))
      (set `local.LocalComplete` _output_get_2)))
  (return (`local.LocalComplete`)))

(fn `UpdateTimes`
  (bind _playercontrollerreference (`self.PlayerControllerReference`))
  ;[1 1 1] Pass gold---bronze times to Player Controller
  (set `/Game/Blueprints/MyPlayerController.GoldTime` (`self.GoldTime`) _playercontrollerreference)
  (set `/Game/Blueprints/MyPlayerController.SilverTime` (`self.SilverTime`) _playercontrollerreference)
  (set `/Game/Blueprints/MyPlayerController.BronzeTime` (`self.BronzeTime`) _playercontrollerreference)
  (set `/Game/Blueprints/MyPlayerController.DefaultBestLapTime` (`self.DefaultBestLap`) _playercontrollerreference)
  (set `/Game/Blueprints/MyPlayerController.DefaultBestRaceTime` (`self.DefaultBestTime`) _playercontrollerreference))

(fn `UserConstructionScript`)