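; Checkpoint actor for a vehicle racing lap system that reports when the player's vehicle passes through it.
; On trigger overlap, it accepts only a VehicleBlueprint whose velocity dotted with the Arrow's forward vector is positive, blocking reverse clears.
; A valid pass fires the CheckpointCleared dispatcher with its checkpoint number, hides the trigger and particle effect, and disables the trigger's overlap events.
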(event `self.Trigger.OnComponentEndOverlap`
  (params (OverlappedComponent :type "PrimitiveComponent Object Reference") (OtherActor :type "Actor Object Reference") (OtherComp :type "PrimitiveComponent Object Reference") (OtherBodyIndex :type Integer))
  ;[0.9593 1 0.1335] Checkpoint System
)

(event `self.Trigger.OnComponentBeginOverlap`
  (params (OverlappedComponent :type "PrimitiveComponent Object Reference") (OtherActor :type "Actor Object Reference") (OtherComp :type "PrimitiveComponent Object Reference") (OtherBodyIndex :type Integer) (bFromSweep :type Boolean) (SweepResult :type "HitResult Structure (by ref)"))
  (bind _trigger (`self.Trigger`))
  ;[0.9593 1 0.1335] Checkpoint System
  ;;[0.398 0.3756 1] Use this instead if you want to clear the checkpoint if player touches the trigger volume at all
  (bind _asvehicle_blueprint (cast `/Game/Blueprints/VehicleBlueprint` OtherActor))
  (if (> (`KismetMathLibrary.Dot_VectorVector` (`self.GetVelocity` _asvehicle_blueprint) (`KismetMathLibrary.Conv_RotatorToVector` (`SceneComponent.K2_GetComponentRotation` (`self.Arrow`)))) 0.0)
    ;;[1 0 0.1144] Call Checkpoint Dispatcher
    (`self.CheckpointCleared` (`self.CheckpointNumber`))
    ;;[0.3854 0.3854 0.3854] Hide components. Just drag the components you'd like to hide after checkpoint clearance in here.
    (`SceneComponent.SetHiddenInGame` _trigger true false)
    (`SceneComponent.SetHiddenInGame` (`self.ParticleSystem`) true false)
    ;;[1 1 1] Temporarily deactivate the checkpoint and activate after lap is completed later on.
    (set `PrimitiveComponent.bGenerateOverlapEvents` false _trigger)))

(fn `UserConstructionScript`)